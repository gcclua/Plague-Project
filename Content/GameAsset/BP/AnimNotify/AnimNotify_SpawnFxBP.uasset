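; Anim notify that spawns an FX Blueprint actor and attaches it to a socket on the animated mesh.
; When the FxBP class is valid, it spawns the actor at Offset with the AttackSocket rotation and given Scale, unless colliding.
; Attachment keeps location and scale as relative values, so Offset becomes a socket-relative offset, and snaps rotation to the socket.
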(fn `Received_Notify`
  (params (MeshComp :type "SkeletalMeshComponent Object Reference") (Animation :type "AnimSequenceBase Object Reference"))
  (returns (ReturnValue :type Boolean))
  (bind _fxbp (`self.FxBP`))
  (if (`KismetSystemLibrary.IsValidClass` _fxbp)
    (bind _returnvalue (`|SpawnActorFromClass` _fxbp (`KismetMathLibrary.MakeTransform` (`self.Offset`) (`SceneComponent.GetSocketRotation` MeshComp (`self.AttackSocket`)) (`self.Scale`)) "DontSpawnIfColliding" "OverrideRootScale" null null))
    (`Actor.K2_AttachToComponent` _returnvalue MeshComp (`self.AttackSocket`) "KeepRelative" "SnapToTarget" "KeepRelative" true)
    (return false)))